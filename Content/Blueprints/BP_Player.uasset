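; BP_Player is the player, a flipbook sprite character with camera-yaw-relative movement and interaction with nearby actors.
; A fast looping timer searches InteractRange for the nearest BPI_Interactable and sends start and end overlap messages as the target changes.
; The Possess input messages the current target and also hides the character sprite.
; A second timer picks directional walk or idle flipbooks from movement input and velocity.
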(event Custom|InteractTick
  (Utilities|FlowControl|Sequence
    (:then_0
      ;[1 1 1] Find And Set Nearest Interactable
      (Variables|Default|SetNearestDist 1e+10)
      (for _array_element (Collision|GetOverlappingActors (Variables|Components|GetInteractRange) 0 :!class /Script/Engine.PrimitiveComponent)
        (if (Utilities|DoesObjectImplementInterface _array_element "/Game/Blueprints/BPI_Interactable.BPI_Interactable_C")
          (if (< (Transformation|GetDistanceTo _array_element) (Variables|Default|GetNearestDist))
            (Variables|Default|SetNearestDist (Transformation|GetDistanceTo _array_element))
            (Variables|Components|SetTempOverlap _array_element)
            (else
              (Variables|Components|SetCurrentOverlap _array_element))))))
    (:then_1
      ;[1 1 1] Is Overlapped currently Overlapping?
      (if (Collision|IsOverlappingActor (Variables|Components|GetInteractRange) (Variables|Components|GetTempOverlap) :!class /Script/Engine.PrimitiveComponent)
        (Variables|Components|SetCurrentOverlap (Variables|Components|GetTempOverlap))
        ;[1 1 1] If Current Target is Old Target, Start Current's Overlap
        (if (== (Variables|Components|GetCurrentOverlap) (Variables|Components|GetOldOverlap))
          (Class|BPIInteractable|StartOverlap(Message) (Variables|Components|GetCurrentOverlap))
          (else
            (Utilities|IsValid (Variables|Components|GetOldOverlap) :!label _label
              (:Is%20Valid
                (Class|BPIInteractable|EndOverlap(Message) (Variables|Components|GetOldOverlap)))
              (:Is%20Not%20Valid
                _))))
        (else
          (Variables|Components|SetCurrentOverlap 0)
          (goto _label)))
      (Variables|Components|SetOldOverlap (Variables|Components|GetCurrentOverlap)))))

(event EventBeginPlay
  (Transformation|AttachActorToActor (Variables|Default|GetCameraRef) self "None" "SnapToTarget" "KeepRelative" "KeepRelative" false)
  (Utilities|Time|SetTimerbyFunctionName 0 "Set Animation" 0.05 true)
  (Utilities|Time|SetTimerbyEvent (delegate Custom|InteractTick) 0.01 true))

(event Input|ActionEvents|InputActionPossess
  (params (Key :type Key%20Structure))
  (:Pressed
    (Rendering|SetVisibility (Variables|Components|GetCharacter) false false)))

(event Input|ActionEvents|InputActionPossess
  (params (Key :type Key%20Structure))
  ;[1 1 1] Interact
  (:Pressed
    (bind _currentoverlap (Variables|Components|GetCurrentOverlap)
      (:then
        (Class|BPIInteractable|Interact(Message) _currentoverlap)
        (Development|PrintString "Hello"))
      (:else
        (Development|PrintString "Not Valid")))))

(event Input|AxisEvents|InputAxisForwardMove
  (params (AxisValue :type Float%20%28single-precision%29))
  (Pawn|Input|AddMovementInput (Math|Vector|GetForwardVector (Math|Rotator|MakeRotator 0.0 0.0 (.yaw (Transformation|GetWorldRotation (Variables|/Game/Blueprints/BP_Camera.BP_Camera_C|GetCamera (Variables|Default|GetCameraRef)))))) AxisValue false)
  (Variables|Default|SetDirVector (Math|Vector2D|MakeVector2D AxisValue (.y (Variables|Default|GetDirVector)))))

(event Input|AxisEvents|InputAxisRightMove
  (params (AxisValue :type Float%20%28single-precision%29))
  (Pawn|Input|AddMovementInput (Math|Vector|GetRightVector (Math|Rotator|MakeRotator 0.0 0.0 (.yaw (Transformation|GetWorldRotation (Variables|/Game/Blueprints/BP_Camera.BP_Camera_C|GetCamera (Variables|Default|GetCameraRef)))))) AxisValue false)
  (Variables|Default|SetDirVector (Math|Vector2D|MakeVector2D (.x (Variables|Default|GetDirVector)) AxisValue)))

(event Input|AxisEvents|InputAxisTurn
  (params (AxisValue :type Float%20%28single-precision%29))
  (Pawn|Input|AddControllerYawInput AxisValue))

(fn ConstructionScript)

(fn SetAnimation
  (if (or (!= (Input|AxisValues|GetForwardMove) 0.0) (!= (Input|AxisValues|GetRightMove) 0.0))
    (Variables|Default|SetAnimEnum (select (< (Input|AxisValues|GetForwardMove) 0.0) "NewEnumerator1" (select (> (Input|AxisValues|GetForwardMove) 0.0) "NewEnumerator0" (select (> (Input|AxisValues|GetRightMove) 0.0) "NewEnumerator2" "NewEnumerator3")))))
  (Sprite|SetFlipbook (Variables|Components|GetCharacter) (select (> (Math|Vector|VectorLength (Transformation|GetVelocity)) 0.0) (Utilities|Select :Index (Variables|Default|GetAnimEnum) :NewEnumerator0 "/Game/Assets/Sprites/TestChar/Idle/up.up" :NewEnumerator1 "/Game/Assets/Sprites/TestChar/Idle/down.down" :NewEnumerator2 "/Game/Assets/Sprites/TestChar/Idle/right.right" :NewEnumerator3 "/Game/Assets/Sprites/TestChar/Idle/left.left") (Utilities|Select :Index (Variables|Default|GetAnimEnum) :NewEnumerator0 "/Game/Assets/Sprites/TestChar/Idle/idle_up.idle_up" :NewEnumerator1 "/Game/Assets/Sprites/TestChar/Idle/idle_down.idle_down" :NewEnumerator2 "/Game/Assets/Sprites/TestChar/Idle/idle_right.idle_right" :NewEnumerator3 "/Game/Assets/Sprites/TestChar/Idle/idle_left.idle_left"))))