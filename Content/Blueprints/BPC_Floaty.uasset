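; BPC_Floaty is a component that plays timed sequences of floating text lines on the player's FloatingText.
; TriggerFloaty collects DT_Floaty rows whose names contain BranchToTrigger, guarded by a DoOnce that resets when the sequence ends.
; A self-chaining timer shows each line after that row's delay.
; Begin and end dispatchers bracket playback, with the text hidden two seconds after the last line.
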(event Custom|TriggerFloaty
  (bind _playerref (Variables|Default|GetPlayerRef))
  (bind _floatingtext (Variables|/Game/Blueprints/Possessables/BP_BasePossessable.BP_BasePossessable_C|GetFloatingText _playerref))
  (Utilities|FlowControl|Sequence
    (:then_0
      ;[1 1 1] Init Dialogue
      (Utilities|FlowControl|DoOnce false :!label _label
        (:Completed
          (Utilities|Array|Clear (Variables|Default|GetBranchesArray))
          (Variables|Default|SetIndex 0)
          (Rendering|Components|TextRender|SetText _floatingtext (Utilities|Text|MakeLiteralText ""))
          (Rendering|SetVisibility _floatingtext true false)
          (bind _outrownames (DataTable|GetDataTableRowNames "/Game/Data/DT_Floaty.DT_Floaty"))
          (for _array_element _outrownames
            (if (Utilities|String|Contains (Utilities|String|ToString(Name) _array_element) (Utilities|String|ToString(Name) (Variables|Default|GetBranchToTrigger)))
              (bind _returnvalue (Utilities|GetDataTableRow "/Game/Data/DT_Floaty.DT_Floaty" _array_element)
                (:then
                  (Utilities|Array|Add (Variables|Default|GetBranchesArray) _returnvalue)
                  (Variables|Default|SetIndex 0)
                  (Variables|Default|SetisEnd false)
                  (Variables|Default|SetIsShowingText true)
                  (Default|CallOnBeginFloaty))))))))
    (:then_1
      (if (Variables|Default|GetisEnd)
        (Utilities|Time|ClearandInvalidateTimerbyHandle (Variables|Default|GetTextTimer))
        (Utilities|FlowControl|Delay 2.0)
        (Variables|Default|SetIsShowingText false)
        (Rendering|SetVisibility (Variables|/Game/Blueprints/Possessables/BP_BasePossessable.BP_BasePossessable_C|GetFloatingText (Variables|Default|GetPlayerRef)) false false)
        (Default|CallOnEndFloaty)
        (goto _label Reset)
        (else
          ;[1 1 1] Iterate through the BranchesArray based on each branch's delay
          (if (<= (.Delay (Utilities|Struct|BreakS_FloatyData (Utilities|Array|Get(acopy) (Variables|Default|GetBranchesArray) (Variables|Default|GetIndex)))) 0.0)
            (Variables|Default|SetCurrentDelay 0.01)
            (else
              (Variables|Default|SetCurrentDelay (.Delay (Utilities|Struct|BreakS_FloatyData (Utilities|Array|Get(acopy) (Variables|Default|GetBranchesArray) (Variables|Default|GetIndex)))))))
          (bind _returnvalue_2 (Utilities|Time|SetTimerbyEvent (delegate Custom|Show%20Floaty%20Text) (Variables|Default|GetCurrentDelay)))
          (Variables|Default|SetTextTimer _returnvalue_2))))))

(event Custom|Show%20Floaty%20Text
  ;[1 1 1] Iterate through the BranchesArray based on each branch's delay
  (Rendering|Components|TextRender|SetText (Variables|/Game/Blueprints/Possessables/BP_BasePossessable.BP_BasePossessable_C|GetFloatingText (Variables|Default|GetPlayerRef)) (Utilities|Text|ToText(String) (.Text (Utilities|Struct|BreakS_FloatyData (Utilities|Array|Get(acopy) (Variables|Default|GetBranchesArray) (Variables|Default|GetIndex))))))
  (Math|Integer|IncrementInt (Variables|Default|GetIndex)
    (:%20%20
      (if (Utilities|Array|IsValidIndex (Variables|Default|GetBranchesArray) (Variables|Default|GetIndex))
        _
        (else
          (Variables|Default|SetisEnd true)))
      (CallFunction|NextFloaty))))

(event Custom|NextFloaty
  (bind _playerref (Variables|Default|GetPlayerRef))
  (bind _floatingtext (Variables|/Game/Blueprints/Possessables/BP_BasePossessable.BP_BasePossessable_C|GetFloatingText _playerref))
  (if (Variables|Default|GetisEnd)
    (Utilities|Time|ClearandInvalidateTimerbyHandle (Variables|Default|GetTextTimer))
    (Utilities|FlowControl|Delay 2.0)
    (Variables|Default|SetIsShowingText false)
    (Rendering|SetVisibility (Variables|/Game/Blueprints/Possessables/BP_BasePossessable.BP_BasePossessable_C|GetFloatingText (Variables|Default|GetPlayerRef)) false false)
    (Default|CallOnEndFloaty)
    ;[1 1 1] Init Dialogue
    (Utilities|FlowControl|DoOnce false) ; enters at Reset
    (else
      ;[1 1 1] Iterate through the BranchesArray based on each branch's delay
      (if (<= (.Delay (Utilities|Struct|BreakS_FloatyData (Utilities|Array|Get(acopy) (Variables|Default|GetBranchesArray) (Variables|Default|GetIndex)))) 0.0)
        (Variables|Default|SetCurrentDelay 0.01)
        (else
          (Variables|Default|SetCurrentDelay (.Delay (Utilities|Struct|BreakS_FloatyData (Utilities|Array|Get(acopy) (Variables|Default|GetBranchesArray) (Variables|Default|GetIndex)))))))
      (bind _returnvalue (Utilities|Time|SetTimerbyEvent (delegate Custom|Show%20Floaty%20Text) (Variables|Default|GetCurrentDelay)))
      (Variables|Default|SetTextTimer _returnvalue))))

(event EventBeginPlay
  (Utilities|FlowControl|Delay 0.1)
  (bind _asbp_player_controller (Utilities|Casting|CastToBP_PlayerController (Game|GetPlayerController 0)))
  (Variables|Default|SetHUDRef (Variables|/Game/Blueprints/BP_PlayerController.BP_PlayerController_C|GetHUDRef _asbp_player_controller))
  (Variables|Default|SetPlayerRef (Variables|/Game/Blueprints/BP_PlayerController.BP_PlayerController_C|GetPlayerRef _asbp_player_controller)))

(event EventTick
  (params (DeltaSeconds :type Float%20%28single-precision%29)))

(fn ShowFloatyText)