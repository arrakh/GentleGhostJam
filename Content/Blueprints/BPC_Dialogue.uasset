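; Dialogue component that plays branching conversations from the DT_Dialogue data table through the player's dialogue widget.
; On BeginPlay it takes the HUD and dialogue references from BP_PlayerController and registers itself with the HUD.
; Each TriggerDialogue call advances one row, with a DoOnce handling opening until closing resets it.
; Rows either show text and set the next branch, or open responses and hide the HUD's ScreenClick.
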(event Custom|CloseDialogue
  (bind _dialogueref (Variables|Default|GetDialogueRef))
  (Default|CloseDialogue (Variables|Default|GetDialogueRef))
  (Variables|Default|SetisInDialogue false)
  (Default|CallOnEndDialogue)
  ;[1 1 1] Init Dialogue
  (Utilities|FlowControl|DoOnce false) ; enters at Reset
)

(event Custom|TriggerDialogue
  (bind _dialogueref (Variables|Default|GetDialogueRef))
  (Utilities|FlowControl|Sequence
    (:then_0
      ;[1 1 1] Init Dialogue
      (Utilities|FlowControl|DoOnce false :!label _label
        (:Completed
          (Default|OpenDialogue _dialogueref)
          (Variables|/Game/UI/WBP_DialogueBox.WBP_DialogueBox_C|SetDiaCompRef _dialogueref self)
          (Variables|Default|SetNextBranch (Variables|Default|GetDefaultBranch))
          (Variables|Default|SetisEnd false)
          (Variables|Default|SetisInDialogue true)
          (Default|CallOnBeginDialogue))))
    (:then_1
      (if (Variables|Default|GetisEnd)
        (Default|CloseDialogue (Variables|Default|GetDialogueRef))
        (Variables|Default|SetisInDialogue false)
        (Default|CallOnEndDialogue)
        (goto _label Reset)
        (else
          (bind _returnvalue (Utilities|GetDataTableRow "/Game/Data/DT_Dialogue.DT_Dialogue" (Variables|Default|GetNextBranch))
            (:then
              (if (not (.HasResponse (Utilities|Struct|BreakS_DialogueData _returnvalue)))
                ;[1 1 1] Set Dialogue
                (Default|SetDialogue (Variables|Default|GetDialogueRef) _returnvalue)
                (Variables|Default|SetisEnd (.isFinalBranch (Utilities|Struct|BreakS_DialogueData _returnvalue)))
                (Variables|Default|SetNextBranch (.NextDialogueBranch (Utilities|Struct|BreakS_DialogueData _returnvalue)))
                (else
                  (Default|OpenResponse (Variables|Default|GetDialogueRef) (.ResponseBranch (Utilities|Struct|BreakS_DialogueData _returnvalue)))
                  (Widget|SetVisibility (Variables|/Game/UI/WBP_HUD.WBP_HUD_C|GetScreenClick (Variables|Default|GetHUDRef)) "Collapsed"))))))))))

(event EventBeginPlay
  (Utilities|FlowControl|Delay 0.1)
  (bind _asbp_player_controller (Utilities|Casting|CastToBP_PlayerController (Game|GetPlayerController 0)))
  (bind _output_get (Variables|Default|SetHUDRef (Variables|/Game/Blueprints/BP_PlayerController.BP_PlayerController_C|GetHUDRef _asbp_player_controller)))
  (Variables|/Game/UI/WBP_HUD.WBP_HUD_C|SetDiaCompRef _output_get self)
  (Variables|Default|SetDialogueRef (Variables|/Game/Blueprints/BP_PlayerController.BP_PlayerController_C|GetDialogueRef _asbp_player_controller)))

(event EventTick
  (params (DeltaSeconds :type Float%20%28single-precision%29)))