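; Base class for possessable pawns that the player takes control of through Interact, with empty movement and camera-turn events for children to override.
; Possessing uses a timeline to glide the shared BP_Camera to the capsule, then attaches it.
; PawnPossess triggers EndInteract, which teleports the stored player to this pawn and sends it InteractMessage.
; A fast looping timer derives a four-way Direction from camera yaw and billboards the Scene component against the camera's forward vector.
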(event Custom|OnPossess
  (Pawn|Possess (Game|GetPlayerController 0) self)
  (bind _lerp (Timeline|PossessLerp PlayFromStart)
    (:Update
      (Transformation|SetActorLocation (Variables|Default|GetCameraRef) (Math|Vector|Lerp(Vector) (Transformation|GetWorldLocation (Variables|/Game/Blueprints/BP_Camera.BP_Camera_C|GetDefaultSceneRoot (Variables|Default|GetCameraRef))) (Transformation|GetWorldLocation (Variables|Default|GetCapsule)) _lerp) false false)
      (Rendering|SetActorHiddenInGame false))
    (:Finished
      (Transformation|AttachActorToActor (Variables|Default|GetCameraRef) self "None" "KeepWorld" "KeepWorld" "KeepRelative" true))))

(event Custom|Pawn%20Move%20Forward
  (params (AxisValue :type Float%20%28single-precision%29))
  ;[1 1 1] Base events to be overridden in child classes
)

(event Custom|Pawn%20Move%20Right
  (params (AxisValue :type Float%20%28single-precision%29))
  ;[1 1 1] Base events to be overridden in child classes
)

(event Custom|Pawn%20Turn%20Camera
  (params (AxisValue :type Float%20%28single-precision%29))
  ;[1 1 1] Base events to be overridden in child classes
)

(event Custom|Pawn%20Possess
  ;[1 1 1] Base events to be overridden in child classes
  (CallFunction|EndInteract))

(event EventBeginPlay
  (bind _outactors (Actor|GetAllActorsOfClass "/Game/Blueprints/BP_Camera.BP_Camera_C"))
  (Variables|Default|SetCameraRef (Utilities|Array|Get(acopy) _outactors))
  (Utilities|Time|SetTimerbyFunctionName 0 "SetDirection" 0.01 true))

(event EventInteract
  (CallFunction|OnPossess))

(event Collision|EventActorBeginOverlap
  (params (OtherActor :type Actor%20Object%20Reference)))

(event EventEndInteract
  (bind _asbp_player_controller (Utilities|Casting|CastToBP_PlayerController (Game|GetPlayerController 0)))
  (bind _playerref (Variables|/Game/Blueprints/BP_PlayerController.BP_PlayerController_C|GetPlayerRef _asbp_player_controller)
    (:then
      (Transformation|SetActorLocationAndRotation _playerref (Transformation|GetActorLocation) (Transformation|GetActorRotation) false true)
      (Class|BPIInteractable|Interact(Message) _playerref)
      (Development|PrintString (Utilities|String|BuildString(Object) "Unpossessing from " "" self)))
    (:else
      (Development|PrintString "Not Valid"))))

(fn ConstructionScript)

(fn SetDirection
  (bind _scene (Variables|Default|GetScene))
  (bind _returnvalue (Transformation|GetWorldLocation _scene))
  (LocalVariables|SetLocalYaw (+ (.yaw (Transformation|GetWorldRotation (Variables|/Game/Blueprints/BP_Camera.BP_Camera_C|GetDefaultSceneRoot (Variables|Default|GetCameraRef)))) 45.0))
  (Variables|Default|SetDirection (select (< (LocalVariables|GetLocalYaw) 0.0) (select (< (LocalVariables|GetLocalYaw) -9e+01) "NewEnumerator0" "NewEnumerator2") (select (> (LocalVariables|GetLocalYaw) 9e+01) "NewEnumerator3" "NewEnumerator1")))
  (Transformation|SetRelativeRotation (Variables|Default|GetScene) (Math|Rotator|FindLookatRotation _returnvalue (+ _returnvalue (* (Math|Vector|GetForwardVector (Variables|/Game/Blueprints/BP_Camera.BP_Camera_C|GetCamera (Variables|Default|GetCameraRef))) -10))) false true))