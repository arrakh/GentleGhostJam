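; BP_Bowl is a possessable bowl item drawn with directional sprites.
; On BeginPlay it fills the DirectionalSprites map for four directions, reusing the front sprite for two and using left and right sprites for the others.
; The PawnTurnCamera axis input adds controller yaw, while Tick and the construction script only call the parent.
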(event EventBeginPlay
  (|CallParentFunction)
  (Variables|Default|SetDirectionalSprites (Utilities|Map|MakeMap "NewEnumerator0" "/Game/Assets/Sprites/Bowl/bowl_front_Sprite.bowl_front_Sprite" "NewEnumerator1" "/Game/Assets/Sprites/Bowl/bowl_front_Sprite.bowl_front_Sprite" "NewEnumerator2" "/Game/Assets/Sprites/Bowl/bowl_left_Sprite.bowl_left_Sprite" "NewEnumerator3" "/Game/Assets/Sprites/Bowl/bowl_right_Sprite.bowl_right_Sprite")))

(event Collision|EventActorBeginOverlap
  (params (OtherActor :type Actor%20Object%20Reference))
  (|CallParentFunction OtherActor) ; This node is disabled and will not be called.\nDrag off pins to build functionality.
)

(event EventTick
  (params (DeltaSeconds :type Float%20%28single-precision%29))
  (|CallParentFunction DeltaSeconds))

(event EventPawnTurnCamera
  (params (AxisValue :type Float%20%28single-precision%29))
  (Pawn|Input|AddControllerYawInput AxisValue))

(fn ConstructionScript
  (|CallParentFunction))