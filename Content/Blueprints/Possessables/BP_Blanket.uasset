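; BP_Blanket is a blanket Blueprint among the game's possessables, currently a shell with no active logic of its own.
; Its ForwardMove, RightMove and Turn axis events, marked as temporary movement, have nothing connected.
; Orphaned nodes hold unused camera-yaw-relative movement through CameraRef and controller yaw turning.
; BeginPlay and overlap events are disabled, and the construction script only calls its parent.
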(event EventBeginPlay
  (|CallParentFunction) ; This node is disabled and will not be called.\nDrag off pins to build functionality.
)

(event Collision|EventActorBeginOverlap
  (params (OtherActor :type Actor%20Object%20Reference))
  (|CallParentFunction OtherActor) ; This node is disabled and will not be called.\nDrag off pins to build functionality.
)

(event Input|AxisEvents|InputAxisForwardMove
  (params (AxisValue :type Float%20%28single-precision%29))
  ;[1 1 1] Temp movement stuff
)

(event Input|AxisEvents|InputAxisRightMove
  (params (AxisValue :type Float%20%28single-precision%29))
  ;[1 1 1] Temp movement stuff
)

(event Input|AxisEvents|InputAxisTurn
  (params (AxisValue :type Float%20%28single-precision%29))
  ;[1 1 1] Temp movement stuff
)

(fn ConstructionScript
  (|CallParentFunction))