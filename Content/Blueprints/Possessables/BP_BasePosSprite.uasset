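; Base Blueprint for possessable sprite actors that can show a different Paper2D sprite per direction.
; When HasDirectionSprites is set, BeginPlay starts a fast looping timer that calls SetSpriteDir in place of using Tick.
; SetSpriteDir looks up the current Direction in the DirectionalSprites map and applies the matching sprite to PaperSprite if an entry exists.
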(event EventBeginPlay
  (|CallParentFunction)
  (if (Variables|Default|GetHasDirectionSprites)
    (Utilities|Time|SetTimerbyFunctionName 0 "SetSpriteDir" 0.01 true)))

(event Collision|EventActorBeginOverlap
  (params (OtherActor :type Actor%20Object%20Reference))
  (|CallParentFunction OtherActor) ; This node is disabled and will not be called.\nDrag off pins to build functionality.
)

(event EventTick
  (params (DeltaSeconds :type Float%20%28single-precision%29)))

(fn ConstructionScript
  (|CallParentFunction))

(fn SetSpriteDir
  (bind _direction (Variables|Default|GetDirection))
  (bind _directionalsprites (Variables|Default|GetDirectionalSprites))
  (bind (_value _returnvalue) (Utilities|Map|Find _directionalsprites _direction))
  (if _returnvalue
    (Rendering|Components|Sprite|SetSprite (Variables|Default|GetPaperSprite) _value)))