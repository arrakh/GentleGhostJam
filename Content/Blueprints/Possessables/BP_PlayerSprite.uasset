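; Player ghost pawn drawn as a directional Paper2D flipbook, which interacts with nearby objects and possesses BP_BasePossessable targets.
; A looping timer scans InteractRange for the nearest BPI_Interactable, sending overlap start and end messages.
; PawnPossess messages that target; for possessables it also hides the ghost and disables WorldStatic collision, letting it fall forever as a hack.
; Other timers pick walk or idle flipbooks from movement axes and velocity, and draw a downward debug trace.
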(event Custom|InteractTick
  (Utilities|FlowControl|Sequence
    (:then_0
      ;[1 1 1] Find And Set Nearest Interactable
      (Variables|Default|SetNearestDist 1e+10)
      (for _array_element (Collision|GetOverlappingActors (Variables|Default|GetInteractRange) 0 :!class /Script/Engine.PrimitiveComponent)
        (if (and (Utilities|DoesObjectImplementInterface _array_element "/Game/Blueprints/BPI_Interactable.BPI_Interactable_C") (not (Actor|ActorHasTag _array_element "Player")))
          (if (< (Transformation|GetDistanceTo _array_element) (Variables|Default|GetNearestDist))
            (Variables|Default|SetNearestDist (Transformation|GetDistanceTo _array_element))
            (Variables|Components|SetTempOverlap _array_element)
            (else
              (Variables|Components|SetCurrentOverlap _array_element))))))
    (:then_1
      ;[1 1 1] Is Overlapped currently Overlapping?
      (if (Collision|IsOverlappingActor (Variables|Default|GetInteractRange) (Variables|Components|GetTempOverlap) :!class /Script/Engine.PrimitiveComponent)
        (Variables|Components|SetCurrentOverlap (Variables|Components|GetTempOverlap))
        ;[1 1 1] If Current Target is Old Target, Start Current's Overlap
        (if (== (Variables|Components|GetCurrentOverlap) (Variables|Components|GetOldOverlap))
          (Class|BPIInteractable|StartOverlap(Message) (Variables|Components|GetCurrentOverlap))
          (else
            (Utilities|IsValid (Variables|Components|GetOldOverlap) :!label _label
              (:Is%20Valid
                (Class|BPIInteractable|EndOverlap(Message) (Variables|Components|GetOldOverlap)))
              (:Is%20Not%20Valid
                _))))
        (else
          (Variables|Components|SetCurrentOverlap 0)
          (goto _label)))
      (Variables|Components|SetOldOverlap (Variables|Components|GetCurrentOverlap)))))

(event Custom|ParticleTick
  (bind _self self)
  (bind _returnvalue (Transformation|GetActorLocation _self))
  (Collision|LineTraceByChannel _returnvalue (+ _returnvalue (* "0, 0,-1.000000" 2e+02)) "TraceTypeQuery1" false 0 "ForOneFrame"))

(event EventBeginPlay
  (|CallParentFunction)
  (Utilities|Time|SetTimerbyFunctionName 0 "Set Animation" 0.05 true)
  (Utilities|Time|SetTimerbyEvent (delegate Custom|InteractTick) 0.01 true)
  (Utilities|Time|SetTimerbyEvent (delegate Custom|ParticleTick) 0.05 true))

(event EventPawnPossess
  ;[1 1 1] Interact, overrides BasePossessable implementation
  (bind _currentoverlap (Variables|Components|GetCurrentOverlap)
    (:then
      (bind _asbp_base_possessable (Utilities|Casting|CastToBP_BasePossessable _currentoverlap)
        (:then
          (Class|BPIInteractable|Interact(Message) _asbp_base_possessable)
          (Development|PrintString (Utilities|String|BuildString(Object) "Possessing " "" _asbp_base_possessable))
          (Rendering|SetActorHiddenInGame true)
          (Collision|SetCollisionResponsetoChannel (Variables|Default|GetCapsule) "ECC_WorldStatic" "ECR_Ignore") ; Note: this is very hacky and involves watching our beloved ghost friend falling to infinity
        )
        (:CastFailed
          (Class|BPIInteractable|Interact(Message) _currentoverlap)
          (Development|PrintString (Utilities|String|BuildString(Object) "" "" _currentoverlap)))))
    (:else
      (Development|PrintString "Not Valid"))))

(fn ConstructionScript
  (|CallParentFunction)
  (Variables|Default|SetIsSetDirection true))

(fn SetAnimation
  (if (or (!= (Variables|Default|GetForwardAxis) 0.0) (!= (Variables|Default|GetRightAxis) 0.0))
    (Variables|Default|SetAnimEnum (select (< (Variables|Default|GetForwardAxis) 0.0) "NewEnumerator1" (select (> (Variables|Default|GetForwardAxis) 0.0) "NewEnumerator0" (select (> (Variables|Default|GetRightAxis) 0.0) "NewEnumerator3" "NewEnumerator2")))))
  (Sprite|SetFlipbook (Variables|Default|GetPaperFlipbook) (select (> (Math|Vector|VectorLength (Transformation|GetVelocity)) 0.0) (Utilities|Select :Index (Variables|Default|GetAnimEnum) :NewEnumerator0 "/Game/Assets/Sprites/TestChar/Idle/up.up" :NewEnumerator1 "/Game/Assets/Sprites/TestChar/Idle/down.down" :NewEnumerator2 "/Game/Assets/Sprites/TestChar/Idle/right.right" :NewEnumerator3 "/Game/Assets/Sprites/TestChar/Idle/left.left") (Utilities|Select :Index (Variables|Default|GetAnimEnum) :NewEnumerator0 "/Game/Assets/Sprites/TestChar/Idle/idle_up.idle_up" :NewEnumerator1 "/Game/Assets/Sprites/TestChar/Idle/idle_down.idle_down" :NewEnumerator2 "/Game/Assets/Sprites/TestChar/Idle/idle_right.idle_right" :NewEnumerator3 "/Game/Assets/Sprites/TestChar/Idle/idle_left.idle_left"))))