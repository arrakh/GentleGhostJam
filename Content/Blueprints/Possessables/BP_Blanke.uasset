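; BP_Blanke is a possessable blueprint, mostly a stub: its Interact event and construction script are empty.
; Its only working logic is SetDirection, which offsets the referenced camera root's world yaw by 45 degrees and buckets it into one of four Direction enum values.
; Default events are disabled, and leftover data-table and look-at rotation nodes are unused.
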(event EventBeginPlay)

(event Collision|EventActorBeginOverlap
  (params (OtherActor :type Actor%20Object%20Reference)))

(event EventTick
  (params (DeltaSeconds :type Float%20%28single-precision%29)))

(event EventInteract)

(fn ConstructionScript)

(fn SetDirection
  (LocalVariables|SetLocalYaw (+ (.yaw (Transformation|GetWorldRotation (Variables|/Game/Blueprints/BP_Camera.BP_Camera_C|GetDefaultSceneRoot (Variables|Default|GetCameraRef)))) 45.0))
  (Variables|Default|SetDirection (select (< (LocalVariables|GetLocalYaw) 0.0) (select (< (LocalVariables|GetLocalYaw) -9e+01) "NewEnumerator0" "NewEnumerator2") (select (> (LocalVariables|GetLocalYaw) 9e+01) "NewEnumerator3" "NewEnumerator1"))))