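; BP_Test is a possessable pawn, apparently a test asset, that handles forward, strafe and camera-turn input events.
; Forward and right movement input follows the yaw of the camera held in CameraRef, ignoring pitch and roll so movement stays horizontal.
; Turn input feeds controller yaw directly, and the default BeginPlay, overlap and Tick events are left disabled.
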(event EventBeginPlay
  (|CallParentFunction) ; This node is disabled and will not be called.\nDrag off pins to build functionality.
)

(event Collision|EventActorBeginOverlap
  (params (OtherActor :type Actor%20Object%20Reference))
  (|CallParentFunction OtherActor) ; This node is disabled and will not be called.\nDrag off pins to build functionality.
)

(event EventTick
  (params (DeltaSeconds :type Float%20%28single-precision%29))
  (|CallParentFunction DeltaSeconds) ; This node is disabled and will not be called.\nDrag off pins to build functionality.
)

(event EventPawnMoveForward
  (params (AxisValue :type Float%20%28single-precision%29))
  (Pawn|Input|AddMovementInput (Math|Vector|GetForwardVector (Math|Rotator|MakeRotator 0.0 0.0 (.yaw (Transformation|GetWorldRotation (Variables|/Game/Blueprints/BP_Camera.BP_Camera_C|GetCamera (Variables|Default|GetCameraRef)))))) AxisValue false))

(event EventPawnMoveRight
  (params (AxisValue :type Float%20%28single-precision%29))
  (Pawn|Input|AddMovementInput (Math|Vector|GetRightVector (Math|Rotator|MakeRotator 0.0 0.0 (.yaw (Transformation|GetWorldRotation (Variables|/Game/Blueprints/BP_Camera.BP_Camera_C|GetCamera (Variables|Default|GetCameraRef)))))) AxisValue false))

(event EventPawnTurnCamera
  (params (AxisValue :type Float%20%28single-precision%29))
  (Pawn|Input|AddControllerYawInput AxisValue))

(fn ConstructionScript
  (|CallParentFunction))