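; BP_HoverComponent is a hover spring that pushes its owning BP_BasePossessable up from the surface below the component.
; While active, a looping timer, rather than Tick, line-traces along the component's down vector to measure compression against HoverDistance, with debug drawing on.
; A spring-damper force is applied to the owner's root primitive at the component's location.
; The damping term divides by frame delta time, not the timer interval.
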(event Custom|TickEvent
  (bind _returnvalue (Transformation|GetWorldLocation))
  (if (Variables|Default|GetisActivate)
    (Utilities|IsValid (Variables|Default|GetParentRef)
      (:Is%20Valid
        (bind (_outhit _returnvalue_2) (Collision|LineTraceByChannel _returnvalue (- _returnvalue (* (Math|Vector|GetUpVector) (Variables|Default|GetHoverDistance))) "TraceTypeQuery1" false 0 "ForDuration" true "(R=1.000000,G=0.000000,B=0.000000,A=1.000000)" "(R=0.000000,G=1.000000,B=0.000000,A=1.000000)" 0.05))
        (if _returnvalue_2
          (bind _output_get (Variables|Default|SetHoverDelta (- (Variables|Default|GetHoverDistance) (.Distance (Collision|BreakHitResult _outhit)))))
          (bind _asprimitive_component (Utilities|Casting|CastToPrimitiveComponent (Variables|/Script/Engine.Actor|GetRootComponent (Variables|Default|GetParentRef))))
          (Class|PrimitiveComponent|AddForceatLocation _asprimitive_component (* (Math|Vector|GetUpVector) (+ (* (/ (- _output_get (Variables|Default|GetPreviousHoverDelta)) (Utilities|Time|GetWorldDeltaSeconds)) (Variables|Default|GetDampingCoefficient)) (* _output_get (Variables|Default|GetSpringCoefficient)))) (Transformation|GetWorldLocation) "None")
          (Variables|Default|SetPreviousHoverDelta (Variables|Default|GetHoverDelta)))))))

(event EventBeginPlay
  (Utilities|Time|SetTimerbyEvent (delegate Custom|TickEvent) 0.05 true)
  (bind _asbp_base_possessable (Utilities|Casting|CastToBP_BasePossessable (Components|GetOwner)))
  (Variables|Default|SetParentRef _asbp_base_possessable))

(event EventTick
  (params (DeltaSeconds :type Float%20%28single-precision%29)))