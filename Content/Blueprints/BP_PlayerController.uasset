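; Player controller that drives whichever BP_BasePossessable pawn it controls and gives it the level's camera.
; On BeginPlay it finds the first BP_Camera and attaches it to that pawn, snapping location and keeping relative rotation and scale.
; Move, turn and Possess inputs cast the current pawn on each event and forward to its functions, leaving the behavior to the pawn.
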(event EventBeginPlay
  (Utilities|FlowControl|Sequence
    (:then_0
      (bind _outactors (Actor|GetAllActorsOfClass "/Game/Blueprints/BP_Camera.BP_Camera_C"))
      (Variables|Default|SetCameraRef (Utilities|Array|Get(acopy) _outactors)))
    (:then_1
      (bind _asbp_base_possessable (Utilities|Casting|CastToBP_BasePossessable (Pawn|GetControlledPawn)))
      (Transformation|AttachActorToActor (Variables|Default|GetCameraRef) _asbp_base_possessable "None" "SnapToTarget" "KeepRelative" "KeepRelative" false))))

(event EventTick
  (params (DeltaSeconds :type Float%20%28single-precision%29)))

(event Input|ActionEvents|InputActionThrustUp
  (params (Key :type Key%20Structure)))

(event Input|ActionEvents|InputActionPossess
  (params (Key :type Key%20Structure))
  (:Pressed
    (bind _asbp_base_possessable (Utilities|Casting|CastToBP_BasePossessable (Pawn|GetControlledPawn)))
    (Default|PawnPossess _asbp_base_possessable)))

(event Input|AxisEvents|InputAxisForwardMove
  (params (AxisValue :type Float%20%28single-precision%29))
  (bind _asbp_base_possessable (Utilities|Casting|CastToBP_BasePossessable (Pawn|GetControlledPawn)))
  (Default|PawnMoveForward _asbp_base_possessable AxisValue))

(event Input|AxisEvents|InputAxisRightMove
  (params (AxisValue :type Float%20%28single-precision%29))
  (bind _asbp_base_possessable (Utilities|Casting|CastToBP_BasePossessable (Pawn|GetControlledPawn)))
  (Default|PawnMoveRight _asbp_base_possessable AxisValue))

(event Input|AxisEvents|InputAxisTurn
  (params (AxisValue :type Float%20%28single-precision%29))
  (bind _asbp_base_possessable (Utilities|Casting|CastToBP_BasePossessable (Pawn|GetControlledPawn)))
  (Default|PawnTurnCamera _asbp_base_possessable AxisValue))

(fn ConstructionScript)